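; BP_EditGameMode is a game mode, apparently for level editing, that creates and places level elements through a factory actor.
; BeginPlay spawns a BP_LevelElementFactory at the origin and stores the reference.
; SpawnLevelElement checks that factory, asks it for three elements and spaces them evenly along X at a fixed height.
; Nothing in this Blueprint calls SpawnLevelElement.
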(event `self.ReceiveBeginPlay`
  (bind _returnvalue (`|SpawnActorFromClass` "/Game/Element/BaseElement/BP_LevelElementFactory.BP_LevelElementFactory_C" (`KismetMathLibrary.MakeTransform` (0.0 0.0 0.0)) "Undefined" "OverrideRootScale" null null))
  (set `self.LevelElementFactory` _returnvalue))

(fn `SpawnLevelElement`
  (bind _levelelementfactory (`self.LevelElementFactory`))
  (`/Engine/EditorBlueprintResources/StandardMacros.IsValid` _levelelementfactory
    (:`Is Valid`
      (for _index (range 3)
        (bind _returnvalue (`LevelElementFactory.CreateLevelElement` _levelelementfactory))
        (`self.K2_SetActorLocation` _returnvalue (`KismetMathLibrary.MakeVector` (* _index 400.0) 0.0 300.0) false false)))))

(fn `UserConstructionScript`)