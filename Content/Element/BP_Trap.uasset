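; BP_Trap is a trap actor that opens when something enters its box trigger and closes when the overlap ends.
; Overlaps send events to a state component that moves between Close, Up, Open and Down states, with Up and Down each playing a sequence.
; Finished sequences settle the trap into Open or Close.
; An interruption mid-motion starts the opposite sequence at the interrupted one's remaining time, so movement reverses from the mirrored point.
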(event `self.ReceiveBeginPlay`
  (add `MovieSceneSequencePlayer.OnFinished` (`ActorSequenceComponent.SequencePlayer` (`self.DownSeq`)) (delegate `CustomEvent_1`))
  (add `MovieSceneSequencePlayer.OnFinished` (`ActorSequenceComponent.SequencePlayer` (`self.UpSeq`)) (delegate `CustomEvent_0`)))

(event `CustomEvent_1`
  (`StateComponent.EnterState` (`self.MyStateComponent`) "CloseState"))

(event `CustomEvent_0`
  (`StateComponent.EnterState` (`self.MyStateComponent`) "OpenState"))

(event `self.Box.OnComponentBeginOverlap`
  (params (OverlappedComponent :type "PrimitiveComponent Object Reference") (OtherActor :type "Actor Object Reference") (OtherComp :type "PrimitiveComponent Object Reference") (OtherBodyIndex :type Integer) (bFromSweep :type Boolean) (SweepResult :type "HitResult Structure (by ref)"))
  (`StateComponent.ExecuteStateEvent` (`self.MyStateComponent`) "OpenTrap"))

(event `self.Box.OnComponentEndOverlap`
  (params (OverlappedComponent :type "PrimitiveComponent Object Reference") (OtherActor :type "Actor Object Reference") (OtherComp :type "PrimitiveComponent Object Reference") (OtherBodyIndex :type Integer))
  (`StateComponent.ExecuteStateEvent` (`self.MyStateComponent`) "CloseTrap"))

(event `self.CloseState_OpenTrap`
  ;[1 1 1] CloseState
  (`StateComponent.EnterState` (`self.MyStateComponent`) "UpState"))

(event `self.UpState_Enter`
  (bind _sequenceplayer (`ActorSequenceComponent.SequencePlayer` (`self.UpSeq`)))
  ;[1 1 1] UpState
  (`MovieSceneSequencePlayer.JumpToSeconds` _sequenceplayer (`self.UpStartTime`))
  (`MovieSceneSequencePlayer.Play` _sequenceplayer)
  (set `self.UpStartTime` 0.0))

(event `self.UpState_CloseTrap`
  (bind _sequenceplayer (`ActorSequenceComponent.SequencePlayer` (`self.UpSeq`)))
  ;[1 1 1] UpState
  (bind _time (`self.GetSeqRemainingTime` _sequenceplayer))
  (set `self.DownStartTime` _time)
  (`MovieSceneSequencePlayer.Stop` _sequenceplayer)
  (`StateComponent.EnterState` (`self.MyStateComponent`) "DownState"))

(event `self.OpenState_Enter`
  ;[1 1 1] OpenState
  (`KismetSystemLibrary.PrintString` "Hello"))

(event `self.OpenState_CloseTrap`
  ;[1 1 1] OpenState
  (`StateComponent.EnterState` (`self.MyStateComponent`) "DownState"))

(event `self.DownState_Enter`
  (bind _sequenceplayer (`ActorSequenceComponent.SequencePlayer` (`self.DownSeq`)))
  ;[1 1 1] DownState
  (`MovieSceneSequencePlayer.JumpToSeconds` _sequenceplayer (`self.DownStartTime`))
  (`MovieSceneSequencePlayer.Play` _sequenceplayer)
  (set `self.DownStartTime` 0.0))

(event `self.DownState_OpenTrap`
  (bind _sequenceplayer (`ActorSequenceComponent.SequencePlayer` (`self.DownSeq`)))
  ;[1 1 1] DownState
  (bind _time (`self.GetSeqRemainingTime` _sequenceplayer))
  (set `self.UpStartTime` _time)
  (`MovieSceneSequencePlayer.Stop` _sequenceplayer)
  (`StateComponent.EnterState` (`self.MyStateComponent`) "UpState"))

(fn `GetSeqRemainingTime`
  (params (SequencePlayer :type "ActorSequencePlayer Object Reference"))
  (returns (Time :type "Float (double-precision)"))
  (return (- (`TimeManagementBlueprintLibrary.Conv_QualifiedFrameTimeToSeconds` (`MovieSceneSequencePlayer.GetEndTime` SequencePlayer)) (`TimeManagementBlueprintLibrary.Conv_QualifiedFrameTimeToSeconds` (`MovieSceneSequencePlayer.GetCurrentTime` SequencePlayer)))))

(fn `UserConstructionScript`)